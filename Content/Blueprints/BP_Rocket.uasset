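; BP_Rocket is a short-lived rocket actor that damages what it overlaps and explodes.
; Overlapping any actor without the Player tag applies fixed damage credited to player controller 0, spawns the explosion effect and 2D sound, then destroys the rocket.
; A lifespan set on BeginPlay removes rockets that hit nothing, and an unconnected delayed-destroy chain never runs.
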(event `self.ReceiveBeginPlay`
  (`self.SetLifeSpan` 3.0))

(event `self.ReceiveActorBeginOverlap`
  (params (OtherActor :type "Actor Object Reference"))
  (if (not (`self.ActorHasTag` OtherActor "Player"))
    (`GameplayStatics.ApplyDamage` OtherActor 10.0 (`GameplayStatics.GetPlayerController` 0) self "/Script/Engine.DamageType")
    (`NiagaraFunctionLibrary.SpawnSystemAtLocation` "/Game/Effects/FX_Explosions/NS_Explosion.NS_Explosion" (`self.K2_GetActorLocation`))
    (`GameplayStatics.SpawnSound2D` "/Game/Sounds/MS_Explosion.MS_Explosion" 1.0 1.0 0.0 null)
    (`self.K2_DestroyActor`)))

(fn `UserConstructionScript`)